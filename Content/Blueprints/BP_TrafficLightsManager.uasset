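; BP_TrafficLightsManager is an unfinished manager for the level's traffic lights, apparently meant to recolor them from a color map.
; On BeginPlay it caches every BP_TraffictLight actor, then prints "No colors" if EmptySetTest returns false.
; EmptySetTest's non-empty checks on the lights and color map are unconnected.
; Recolor is an empty, never-called event, and the CurrentColor lookup in ColorSettings is unused.
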(event `self.ReceiveBeginPlay`
  (bind _outactors (`GameplayStatics.GetAllActorsOfClass` "/Game/Blueprints/BP_TraffictLight.BP_TraffictLight_C"))
  (set `self.TrafficLight` _outactors)
  (if (not (`self.EmptySetTest`))
    (`KismetSystemLibrary.PrintString` "No colors" true true (struct :`G` 0.66 :`B` 1.0 :`A` 1.0) 10.0)))

(event `Recolor`)

(fn `UserConstructionScript`)